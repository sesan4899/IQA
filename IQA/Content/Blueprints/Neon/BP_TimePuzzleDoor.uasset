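; Door actor for a time puzzle that slides open once three puzzle orb flags are all set.
; CheckIndex tests the first three PuzzleOrbs entries and, when all are true, calls OpenDoor and DoorIsUnlocked on the BP_TimePuzzle actors in Orbs.
; OpenDoor plays a timeline whose vector track drives the Door component's relative location.
; The flags are not written in this graph, and nothing here closes the door.
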(event `Open Door`
  (bind (_direction _newtrack_1) (`Timeline|Timeline_0`)
    (:`Update`
      (`SceneComponent.K2_SetRelativeLocation` (`self.Door`) _newtrack_1 false false))))

(event `CheckIndex`
  (bind _puzzle_orbs (`self.Puzzle Orbs`))
  (if (and (`|GetArrayItem` _puzzle_orbs) (`|GetArrayItem` _puzzle_orbs 1) (`|GetArrayItem` _puzzle_orbs 2))
    (`self.Open Door`)
    (for _array_element (`self.Orbs`)
      (bind _asbp_time_puzzle (cast `/Game/Blueprints/Neon/BP_TimePuzzle` _array_element))
      (`/Game/Blueprints/Neon/BP_TimePuzzle.DoorIsUnlocked` _asbp_time_puzzle))))

(fn `UserConstructionScript`)