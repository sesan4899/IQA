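; BP_TargetDoor is a door that a linked switch opens temporarily when the switch is hit.
; On BeginPlay it binds OpenDoor to the switch's hit event, which acts only for its own switch while IsLocked is true.
; One timeline moves the door and clears IsLocked.
; A six-second delay, triggered from that timeline's updates, then plays a second timeline in reverse to move the door again and relock it.
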(event `self.ReceiveBeginPlay`
  (add `/Game/Blueprints/Neon/BP_DoorTarget.SwitchHit` (`self.Switch`) (delegate `OpenDoor`)))

(event `OpenDoor`
  (params (Switch :type "/Game/Blueprints/Neon/BP_DoorTarget Object Reference"))
  (if (== Switch (`self.Switch`))
    (if (`self.IsLocked`)
      (bind (_direction _newtrack_0) (`Timeline|Timeline_0` :!via `PlayFromStart`)
        (:`Update`
          (`SceneComponent.K2_SetRelativeLocation` (`self.Door`) _newtrack_0 false false)
          (set `self.IsLocked` false)
          (`KismetSystemLibrary.Delay` 6.0)
          (bind (_direction_2 _newtrack_0_2) (`Timeline|Timeline_2` :!via `ReverseFromEnd`)
            (:`Update`
              (`SceneComponent.K2_SetRelativeLocation` (`self.Door`) _newtrack_0_2 false false)
              (set `self.IsLocked` true))))))))

(fn `UserConstructionScript`)