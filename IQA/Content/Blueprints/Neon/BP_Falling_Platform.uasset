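; Neon platform Blueprint that turns red and falls shortly after something overlaps its trigger box.
; The box overlap swaps the mesh to a red glow material, waits briefly, then enables physics simulation.
; ResetPosition restores the world location saved at BeginPlay, stops physics and applies a purple glow material, leaving rotation untouched.
; An unconnected looping material-swap chain never runs.
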(event `self.ReceiveBeginPlay`
  (set `self.World Location` (`SceneComponent.K2_GetComponentLocation` (`self.StaticMesh`))))

(event `self.Box.OnComponentBeginOverlap`
  (params (OverlappedComponent :type "PrimitiveComponent Object Reference") (OtherActor :type "Actor Object Reference") (OtherComp :type "PrimitiveComponent Object Reference") (OtherBodyIndex :type Integer) (bFromSweep :type Boolean) (SweepResult :type "HitResult Structure (by ref)"))
  (`PrimitiveComponent.SetMaterial` (`self.StaticMesh`) 0 "/Game/Materials/Neon_Materials/M_GlowEnhanced_red.M_GlowEnhanced_red")
  (`KismetSystemLibrary.Delay` 0.5)
  (`PrimitiveComponent.SetSimulatePhysics` (`self.StaticMesh`) true))

(event `ResetPosition`
  (`SceneComponent.K2_SetWorldLocation` (`self.StaticMesh`) (`self.World Location`) false false)
  (`PrimitiveComponent.SetSimulatePhysics` (`self.StaticMesh`) false)
  (`PrimitiveComponent.SetMaterial` (`self.StaticMesh`) 0 "/Game/Materials/Neon_Materials/M_GlowEnhanced_purple2.M_GlowEnhanced_purple2"))

(fn `UserConstructionScript`)