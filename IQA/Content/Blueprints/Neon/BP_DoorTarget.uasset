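; BP_DoorTarget is a damage-triggered switch target made of three spheres, presumably used to operate a door.
; Any damage while it is unswitched turns all spheres to a hologram material, fires the SwitchHit dispatcher with itself and sets the Switched flag.
; After a fixed delay it restores each sphere's own green, blue or red material and clears the flag so it can be hit again.
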(event `self.ReceiveAnyDamage`
  (params (Damage :type "Float (single-precision)") (DamageType :type "DamageType Object Reference") (InstigatedBy :type "Controller Object Reference") (DamageCauser :type "Actor Object Reference"))
  (if (not (`self.Switched`))
    (`PrimitiveComponent.SetMaterial` (`self.Sphere`) 0 "/Game/Materials/Neon_Materials/M_Hologram_Inst.M_Hologram_Inst")
    (`PrimitiveComponent.SetMaterial` (`self.Sphere1`) 0 "/Game/Materials/Neon_Materials/M_Hologram_Inst.M_Hologram_Inst")
    (`PrimitiveComponent.SetMaterial` (`self.Sphere2`) 0 "/Game/Materials/Neon_Materials/M_Hologram_Inst.M_Hologram_Inst")
    (`self.SwitchHit` self)
    (set `self.Switched` true)
    (`KismetSystemLibrary.Delay` 14.0)
    (`PrimitiveComponent.SetMaterial` (`self.Sphere`) 0 "/Game/Materials/M_Green.M_Green")
    (`PrimitiveComponent.SetMaterial` (`self.Sphere1`) 0 "/Game/Materials/EBlue.EBlue")
    (`PrimitiveComponent.SetMaterial` (`self.Sphere2`) 0 "/Game/Materials/ERed.ERed")
    (set `self.Switched` false)))

(fn `UserConstructionScript`)