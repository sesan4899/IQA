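; A weapon pickup actor that spins and bobs until an overlap triggers it.
; Tick rotates the cylinder and plays a Floating timeline to offset it.
; Overlap casts player pawn 0, not the overlapping actor, to BP_Player and calls WeaponPickup.
; It then loops over Platforms to unhide them and enable collision, with turret revival, activation and the pickup's DestroyActor call all inside that loop body.
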(event `self.ReceiveTick`
  (params (DeltaSeconds :type "Float (single-precision)"))
  ;[1 1 1] Animation
  (`SceneComponent.K2_AddWorldRotation` (`self.Cylinder`) (struct :`Yaw` 0.6) false false)
  (bind (_direction _floating) (`Timeline|Floating`)
    (:`Update`
      (`SceneComponent.K2_AddLocalOffset` (`self.Cylinder`) (`KismetMathLibrary.MakeVector` 0.0 _floating) false false))))

(event `self.ReceiveActorBeginOverlap`
  (params (OtherActor :type "Actor Object Reference"))
  (bind _asbp_player (cast `/Game/Blueprints/Player/BP_Player` (`GameplayStatics.GetPlayerPawn` 0)))
  (`/Game/Blueprints/Player/BP_Player.WeaponPickup` _asbp_player)
  (for _array_element (`self.Platforms`)
    (`self.SetActorHiddenInGame` _array_element false)
    (`PrimitiveComponent.SetCollisionEnabled` (`self.GetComponentByClass` _array_element "/Script/Engine.PrimitiveComponent") "QueryAndPhysics")
    (bind _outactors (`GameplayStatics.GetAllActorsOfClass` "/Game/Blueprints/Enemy/BP_Turret.BP_Turret_C"))
    (for _array_element_2 _outactors
      (set `/Game/Blueprints/Enemy/BP_Turret.Dead` false _array_element_2)
      (`/Game/Blueprints/Enemy/BP_Turret.TurretActivation` _array_element_2))
    (`self.K2_DestroyActor`)))

(fn `UserConstructionScript`)