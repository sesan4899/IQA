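; Second neon bridge actor that reveals four hidden platforms in sequence once the player can trigger it.
; A Bridge3 event from BP_DoubleJump enables the trigger, whose overlap fires the RemoveBridge dispatcher and starts staggered delays.
; Each delay unhides a platform and plays a timeline, then enables query collision and applies blue glow.
; Only the first timeline animates the shared rainbow-fade parameter per update; the others set it on finish.
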(event `self.ReceiveBeginPlay`
  (bind _outactors (`GameplayStatics.GetAllActorsOfClass` "/Game/Blueprints/Neon/BP_DoubleJump.BP_DoubleJump_C"))
  (add `/Game/Blueprints/Neon/BP_DoubleJump.Bridge3` _outactors (delegate `CustomEvent_0`)))

(event `CustomEvent_0`
  (`PrimitiveComponent.SetCollisionEnabled` (`self.Trigger`) "QueryOnly"))

(event `self.Trigger.OnComponentBeginOverlap`
  (params (OverlappedComponent :type "PrimitiveComponent Object Reference") (OtherActor :type "Actor Object Reference") (OtherComp :type "PrimitiveComponent Object Reference") (OtherBodyIndex :type Integer) (bFromSweep :type Boolean) (SweepResult :type "HitResult Structure (by ref)"))
  (bind _platorms (`self.Platorms`))
  (bind _output (`|GetArrayItem` _platorms 2))
  (bind _output_2 (`|GetArrayItem` _platorms))
  (bind _output_3 (`|GetArrayItem` _platorms 3))
  (bind _output_4 (`|GetArrayItem` _platorms 1))
  (bind _returnvalue (`self.GetComponentByClass` _output_4 "/Script/Engine.PrimitiveComponent"))
  (bind _returnvalue_2 (`self.GetComponentByClass` _output "/Script/Engine.PrimitiveComponent"))
  (bind _returnvalue_3 (`self.GetComponentByClass` _output_3 "/Script/Engine.PrimitiveComponent"))
  (bind _returnvalue_4 (`self.GetComponentByClass` _output_2 "/Script/Engine.PrimitiveComponent"))
  (`|ExecutionSequence`
    (:`then_0`
      (`KismetSystemLibrary.Delay` 3.0)
      (`self.SetActorHiddenInGame` _output_2 false)
      (bind (_direction _materialshift) (`Timeline|Timeline_0`)
        (:`Update`
          (`KismetMaterialLibrary.SetScalarParameterValue` "/Game/Materials/Neon_Materials/M_RainbowFade_Coll.M_RainbowFade_Coll" "Amount" _materialshift))
        (:`Finished`
          (`PrimitiveComponent.SetCollisionEnabled` _returnvalue_4 "QueryOnly")
          (`PrimitiveComponent.SetMaterial` _returnvalue_4 0 "/Game/Materials/Neon_Materials/M_GlowEnhanced_blue.M_GlowEnhanced_blue"))))
    (:`then_1`
      (`KismetSystemLibrary.Delay` 3.7)
      (`self.SetActorHiddenInGame` _output_4 false)
      (bind (_direction_2 _materialshift_2) (`Timeline|Timeline_1`)
        (:`Finished`
          (`KismetMaterialLibrary.SetScalarParameterValue` "/Game/Materials/Neon_Materials/M_RainbowFade_Coll.M_RainbowFade_Coll" "Amount" _materialshift_2)
          (`PrimitiveComponent.SetCollisionEnabled` _returnvalue "QueryOnly")
          (`PrimitiveComponent.SetMaterial` _returnvalue 0 "/Game/Materials/Neon_Materials/M_GlowEnhanced_blue.M_GlowEnhanced_blue"))))
    (:`then_2`
      (`KismetSystemLibrary.Delay` 4.5)
      (`self.SetActorHiddenInGame` _output false)
      (bind (_direction_3 _materialshift_3) (`Timeline|Timeline_2`)
        (:`Finished`
          (`KismetMaterialLibrary.SetScalarParameterValue` "/Game/Materials/Neon_Materials/M_RainbowFade_Coll.M_RainbowFade_Coll" "Amount" _materialshift_3)
          (`PrimitiveComponent.SetCollisionEnabled` _returnvalue_2 "QueryOnly")
          (`PrimitiveComponent.SetMaterial` _returnvalue_2 0 "/Game/Materials/Neon_Materials/M_GlowEnhanced_blue.M_GlowEnhanced_blue"))))
    (:`then_3`
      (`self.Remove Bridge`))
    (:`then_4`
      (`KismetSystemLibrary.Delay` 5.2)
      (`self.SetActorHiddenInGame` _output_3 false)
      (bind (_direction_4 _materialshift_4) (`Timeline|Timeline_3`)
        (:`Finished`
          (`KismetMaterialLibrary.SetScalarParameterValue` "/Game/Materials/Neon_Materials/M_RainbowFade_Coll.M_RainbowFade_Coll" "Amount" _materialshift_4)
          (`PrimitiveComponent.SetCollisionEnabled` _returnvalue_3 "QueryOnly")
          (`PrimitiveComponent.SetMaterial` _returnvalue_3 0 "/Game/Materials/Neon_Materials/M_GlowEnhanced_blue.M_GlowEnhanced_blue"))))))

(fn `UserConstructionScript`)