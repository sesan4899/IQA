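; BP_SplinePlatform is a moving platform that travels along a spline when BP_Player enters its trigger box.
; The overlap plays a timeline whose track, scaled by spline length, sets the static mesh's world location along the spline without sweeping.
; Mesh yaw is set on BeginPlay and every update, always sampled at distance zero, so it keeps the spline's starting heading instead of following curves.
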(event `self.ReceiveBeginPlay`
  (bind (_returnvalue_roll _returnvalue_pitch _returnvalue_yaw) (`KismetMathLibrary.BreakRotator` (`SplineComponent.GetRotationAtDistanceAlongSpline` (`self.Spline`) 0.0 "Local")))
  (`SceneComponent.K2_SetRelativeRotation` (`self.StaticMesh`) (`KismetMathLibrary.MakeRotator` 0.0 0.0 _returnvalue_yaw) false false))

(event `self.Box.OnComponentBeginOverlap`
  (params (OverlappedComponent :type "PrimitiveComponent Object Reference") (OtherActor :type "Actor Object Reference") (OtherComp :type "PrimitiveComponent Object Reference") (OtherBodyIndex :type Integer) (bFromSweep :type Boolean) (SweepResult :type "HitResult Structure (by ref)"))
  (bind _staticmesh (`self.StaticMesh`))
  (bind _spline (`self.Spline`))
  (bind (_returnvalue_roll _returnvalue_pitch _returnvalue_yaw) (`KismetMathLibrary.BreakRotator` (`SplineComponent.GetRotationAtDistanceAlongSpline` _spline 0.0 "Local")))
  (cast `/Game/Blueprints/Player/BP_Player` OtherActor)
  (bind (_direction _newtrack_1) (`Timeline|Timeline_0`)
    (:`Update`
      (`SceneComponent.K2_SetWorldLocation` _staticmesh (`SplineComponent.GetLocationAtDistanceAlongSpline` _spline (* _newtrack_1 (`SplineComponent.GetSplineLength` (`self.Spline`))) "World") false false)
      (`SceneComponent.K2_SetRelativeRotation` _staticmesh (`KismetMathLibrary.MakeRotator` 0.0 0.0 _returnvalue_yaw) false false))))

(fn `UserConstructionScript`)