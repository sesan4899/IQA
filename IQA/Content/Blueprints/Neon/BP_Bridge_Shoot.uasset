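; BP_Bridge_Shoot is a shootable trigger that reacts to any damage and signals a bridge event.
; Each hit sets its three spheres to a gold material, then a DoOnce lets only the first hit call the Bridge2 dispatcher.
; An unconnected sequence that would unhide three Platforms actors with staggered delays remains in the graph but never runs.
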(event `self.ReceiveAnyDamage`
  (params (Damage :type "Float (single-precision)") (DamageType :type "DamageType Object Reference") (InstigatedBy :type "Controller Object Reference") (DamageCauser :type "Actor Object Reference"))
  (`PrimitiveComponent.SetMaterial` (`self.Sphere`) 0 "/Game/Materials/M_Gold.M_Gold")
  (`PrimitiveComponent.SetMaterial` (`self.Sphere1`) 0 "/Game/Materials/M_Gold.M_Gold")
  (`PrimitiveComponent.SetMaterial` (`self.Sphere2`) 0 "/Game/Materials/M_Gold.M_Gold")
  (`/Engine/EditorBlueprintResources/StandardMacros.DoOnce` false
    (:`Completed`
      (`self.Bridge2`))))

(fn `UserConstructionScript`)