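; BP_RichardFace is a face actor that slowly turns its Arrow component to look at the first player's pawn.
; Every Tick sets the Arrow's world rotation from Look, which eases the current rotation toward a look-at rotation aimed at the pawn's location.
; The interpolation uses a fixed delta time instead of frame time, so the turn speed depends on frame rate.
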(event `self.ReceiveTick`
  (params (DeltaSeconds :type "Float (single-precision)"))
  (`SceneComponent.K2_SetWorldRotation` (`self.Arrow`) (`self.Look`) false false))

(fn `Look`
  (returns (ReturnValue :type "Rotator Structure"))
  (bind _arrow (`self.Arrow`))
  (return (`KismetMathLibrary.RInterpTo` (`SceneComponent.K2_GetComponentRotation` _arrow) (`KismetMathLibrary.FindLookAtRotation` (`SceneComponent.K2_GetComponentLocation` _arrow) (`self.K2_GetActorLocation` (`GameplayStatics.GetPlayerPawn` 0))) 1.0 0.04)))

(fn `UserConstructionScript`)