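; Damageable puzzle orb that alternates between red and green at random intervals to help open a linked BP_TimePuzzleDoor.
; Damage on green turns it blue for a timed window, adds an entry to the door's PuzzleOrbs array and triggers its check.
; Damage on red or blue removes an entry, red also scheduling a fixed-delay green.
; DoorIsUnlocked makes the orb ignore damage and stops the cycle at blue.
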(event `self.ReceiveBeginPlay`
  (`self.Change to Red`))

(event `self.ReceiveAnyDamage`
  (params (Damage :type "Float (single-precision)") (DamageType :type "DamageType Object Reference") (InstigatedBy :type "Controller Object Reference") (DamageCauser :type "Actor Object Reference"))
  (if (not (`self.DoorUnlock`))
    (switch `int` (`self.MaterialIndex`)
      (:`0`
        (`self.Hit Red`))
      (:`1`
        (`self.HitGreen`))
      (:`2`
        (`self.Hit Blue`)))))

(event `DoorIsUnlocked`
  (set `self.DoorUnlock` true))

(event `Hit Blue`
  (`self.Change to Red`))

(event `Change Material`
  (`PrimitiveComponent.SetMaterial` (`self.Orb`) 0 (`|GetArrayItem` (`self.Materials`) (`self.MaterialIndex`))))

(event `Hit Red`
  (`self.Remove Orb`)
  (`KismetSystemLibrary.K2_SetTimerDelegate` (delegate `Change to Green`) 6.0))

(event `Change to Green`
  (set `self.MaterialIndex` 1)
  (`self.Change Material`)
  (`KismetSystemLibrary.K2_SetTimerDelegate` (delegate `Change to Red`) (`KismetMathLibrary.RandomFloatInRange` 1.0 4.0)))

(event `HitGreen`
  (`self.Add Orb`)
  (set `self.MaterialIndex` 2)
  (`self.Change Material`)
  (set `self.Unlocked` true)
  (if (not (`self.DoorUnlock`))
    (`KismetSystemLibrary.K2_SetTimerDelegate` (delegate `Change to Red`) 6.0)))

(event `Add Orb`
  (bind _asbp_time_puzzle_door (cast `/Game/Blueprints/Neon/BP_TimePuzzleDoor` (`self.Door`)))
  (`KismetArrayLibrary.Array_Add` (`/Game/Blueprints/Neon/BP_TimePuzzleDoor.Puzzle Orbs` _asbp_time_puzzle_door) true)
  (`/Game/Blueprints/Neon/BP_TimePuzzleDoor.CheckIndex` _asbp_time_puzzle_door))

(event `Change to Red`
  (`self.Remove Orb`)
  (if (`self.DoorUnlock`)
    (set `self.MaterialIndex` 2)
    (`self.Change Material`)
    (else
      (set `self.Unlocked` false)
      (set `self.MaterialIndex` 0)
      (`self.Change Material`)
      (`KismetSystemLibrary.K2_SetTimerDelegate` (delegate `Change to Green`) (`KismetMathLibrary.RandomFloatInRange` 1.0 4.0)))))

(event `Remove Orb`
  (bind _asbp_time_puzzle_door (cast `/Game/Blueprints/Neon/BP_TimePuzzleDoor` (`self.Door`)))
  (`KismetArrayLibrary.Array_Remove` (`/Game/Blueprints/Neon/BP_TimePuzzleDoor.Puzzle Orbs` _asbp_time_puzzle_door) (`self.OrbIndex`)))

(fn `UserConstructionScript`)