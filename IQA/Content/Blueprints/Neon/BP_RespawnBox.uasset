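; BP_RespawnBox is a checkpoint volume that, on any actor overlap, sets itself as the player's RespawnPoint.
; Its RespawnEnemies event destroys the listed enemies, spawns live BP_Turrets at their saved locations and moves listed platforms back to their StartPoint.
; StoreLocation is never cleared, and new turrets are not added back to the RespawnEnemies array because that Add node is unconnected.
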(event `self.ReceiveActorBeginOverlap`
  (params (OtherActor :type "Actor Object Reference"))
  (bind _asbp_player (cast `/Game/Blueprints/Player/BP_Player` (`GameplayStatics.GetPlayerPawn` 0)))
  (set `/Game/Blueprints/Player/BP_Player.Respawn point` self _asbp_player))

(event `Respawn Enemies`
  (for _array_element (`self.RespawnEnemies`)
    (`KismetArrayLibrary.Array_Add` (`self.StoreLocation`) (`self.K2_GetActorLocation` _array_element))
    (`self.K2_DestroyActor` _array_element)
    (`KismetSystemLibrary.PrintString` "Destroyed"))
  (for _array_element_2 (`self.StoreLocation`)
    (bind _returnvalue (`|SpawnActorFromClass` "/Game/Blueprints/Enemy/BP_Turret.BP_Turret_C" (`KismetMathLibrary.MakeTransform` _array_element_2) "Undefined" "OverrideRootScale" null null))
    (set `/Game/Blueprints/Enemy/BP_Turret.Dead` false _returnvalue))
  (for _array_element_3 (`self.ResetPlatforms`)
    (bind _asbp_moving_platform (cast `/Game/Blueprints/Neon/BP_MovingPlatform` _array_element_3))
    (`self.K2_SetActorLocation` _array_element_3 (`self.K2_GetActorLocation` (`/Game/Blueprints/Neon/BP_MovingPlatform.StartPoint` _asbp_moving_platform)) false false)))

(fn `UserConstructionScript`)