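; BP_First_Bridge is a bridge actor whose seven static mesh segments appear one after another when triggered.
; On BeginPlay it finds BP_Bridge_Shoot actors and binds its OneTime event to their Bridge2 dispatcher.
; OneTime uses a Sequence with staggered Delays to unhide each segment at half-second intervals.
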(event `self.ReceiveBeginPlay`
  (bind _outactors (`GameplayStatics.GetAllActorsOfClass` "/Game/Blueprints/Neon/BP_Bridge_Shoot.BP_Bridge_Shoot_C"))
  (add `/Game/Blueprints/Neon/BP_Bridge_Shoot.Bridge2` _outactors (delegate `OneTime`)))

(event `OneTime`
  (`|ExecutionSequence`
    (:`then_0`
      (`SceneComponent.SetHiddenInGame` (`self.StaticMesh`) false false))
    (:`then_1`
      (`KismetSystemLibrary.Delay` 0.5)
      (`SceneComponent.SetHiddenInGame` (`self.StaticMesh1`) false false))
    (:`then_2`
      (`KismetSystemLibrary.Delay` 1.0)
      (`SceneComponent.SetHiddenInGame` (`self.StaticMesh2`) false false))
    (:`then_3`
      (`KismetSystemLibrary.Delay` 1.5)
      (`SceneComponent.SetHiddenInGame` (`self.StaticMesh3`) false false))
    (:`then_4`
      (`KismetSystemLibrary.Delay` 2.0)
      (`SceneComponent.SetHiddenInGame` (`self.StaticMesh4`) false false))
    (:`then_5`
      (`KismetSystemLibrary.Delay` 2.5)
      (`SceneComponent.SetHiddenInGame` (`self.StaticMesh5`) false false))
    (:`then_6`
      (`KismetSystemLibrary.Delay` 3.0)
      (`SceneComponent.SetHiddenInGame` (`self.StaticMesh6`) false false))))

(fn `UserConstructionScript`)