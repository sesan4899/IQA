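; BP_Target is a damageable target that transforms a linked PlatformTarget actor when hit.
; Any damage turns its three spheres gold and gives the platform a rainbow fade material, animated by a timeline through a Material Parameter Collection.
; When the timeline finishes, the platform switches to query-only collision and an enhanced glow material.
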(event `self.ReceiveAnyDamage`
  (params (Damage :type "Float (single-precision)") (DamageType :type "DamageType Object Reference") (InstigatedBy :type "Controller Object Reference") (DamageCauser :type "Actor Object Reference"))
  (bind _returnvalue (`self.GetComponentByClass` (`self.PlatformTarget`) "/Script/Engine.PrimitiveComponent"))
  (`PrimitiveComponent.SetMaterial` (`self.Sphere`) 0 "/Game/Materials/M_Gold.M_Gold")
  (`PrimitiveComponent.SetMaterial` (`self.Sphere1`) 0 "/Game/Materials/M_Gold.M_Gold")
  (`PrimitiveComponent.SetMaterial` (`self.Sphere2`) 0 "/Game/Materials/M_Gold.M_Gold")
  (`PrimitiveComponent.SetMaterial` _returnvalue 0 "/Game/Materials/Neon_Materials/M_RainbowFade_Inst.M_RainbowFade_Inst")
  (bind (_direction _materialshift) (`Timeline|Timeline_2`)
    (:`Update`
      (`KismetMaterialLibrary.SetScalarParameterValue` "/Game/Materials/Neon_Materials/M_RainbowFade_Coll.M_RainbowFade_Coll" "Amount" _materialshift))
    (:`Finished`
      (`PrimitiveComponent.SetCollisionEnabled` _returnvalue "QueryOnly")
      (`PrimitiveComponent.SetMaterial` _returnvalue 0 "/Game/Materials/Neon_Materials/M_GlowEnhanced_Inst.M_GlowEnhanced_Inst"))))

(fn `UserConstructionScript`)