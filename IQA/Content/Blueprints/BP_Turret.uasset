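; Enemy turret that sweeps back and forth until the player enters its detection sphere, then tracks and shoots them.
; Tick drives both idle rotation and aiming in fixed per-frame steps, independent of delta time.
; A line trace confirms visibility, and a Gate keeps a single delayed loop spawning projectiles with sound and muzzle flash.
; Damage depletes health until the turret explodes and its parts detach as physics debris.
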(event `self.ReceiveBeginPlay`
  (`SphereComponent.SetSphereRadius` (`self.Targeting`) (`self.DetectionRadius`) true))

(event `self.ReceiveAnyDamage`
  (params (Damage :type "Float (single-precision)") (DamageType :type "DamageType Object Reference") (InstigatedBy :type "Controller Object Reference") (DamageCauser :type "Actor Object Reference"))
  ;[1 1 1] Damage
  (bind _output_get (set `self.Health` (- (`self.Health`) Damage)))
  (if (<= _output_get 0.0)
    (if (not (`self.Dead`))
      (set `self.Dead` true)
      (`self.Die`))))

(event `Die`
  ;[1 1 1] Death
  (`GameplayStatics.SpawnEmitterAtLocation` "/Game/Misc/StarterContent/Particles/P_Explosion.P_Explosion" (`self.K2_GetActorLocation` self))
  (`self.Detach Parts`)
  (`ActorComponent.K2_DestroyComponent` (`self.Sphere`)))

(event `self.Targeting.OnComponentBeginOverlap`
  (params (OverlappedComponent :type "PrimitiveComponent Object Reference") (OtherActor :type "Actor Object Reference") (OtherComp :type "PrimitiveComponent Object Reference") (OtherBodyIndex :type Integer) (bFromSweep :type Boolean) (SweepResult :type "HitResult Structure (by ref)"))
  ;[1 1 1] Target Checking
  (if (== OtherActor (`GameplayStatics.GetPlayerPawn` 0))
    (set `self.Sighted` true)))

(event `self.Targeting.OnComponentEndOverlap`
  (params (OverlappedComponent :type "PrimitiveComponent Object Reference") (OtherActor :type "Actor Object Reference") (OtherComp :type "PrimitiveComponent Object Reference") (OtherBodyIndex :type Integer))
  ;[1 1 1] Target Checking
  (if (== OtherActor (`GameplayStatics.GetPlayerPawn` 0))
    (set `self.Sighted` false)))

(event `self.ReceiveTick`
  (params (DeltaSeconds :type "Float (single-precision)"))
  (bind _sphere (`self.Sphere`))
  (bind _bulletspawn (`self.BulletSpawn`))
  ;[1 1 1] AI
  ;;[1 1 1] Checking
  (if (not (`self.Dead`))
    (bind _asbp_player (cast `/Game/Blueprints/BP_Player` (`GameplayStatics.GetPlayerPawn` 0)))
    (if (not (`/Game/Blueprints/BP_Player.isDead` _asbp_player))
      (if (`self.Sighted`)
        ;;[1 1 1] Shoot
        (`SceneComponent.K2_SetWorldRotation` (`self.Sphere`) (`self.PointTowardsPlayer`) false false)
        (if (`self.CanSeePlayer`)
          (`/Engine/EditorBlueprintResources/StandardMacros.Gate` false :!label _label
            (:`Exit`
              (`|ExecutionSequence`
                (:`then_0`
                  (goto _label :!via `Close`))
                (:`then_1`
                  (`|SpawnActorFromClass` "/Game/Blueprints/BP_Projectile_Enemy.BP_Projectile_Enemy_C" (`KismetMathLibrary.MakeTransform` (`SceneComponent.K2_GetComponentLocation` _bulletspawn) (`SceneComponent.K2_GetComponentRotation` _bulletspawn)) "Undefined" "OverrideRootScale" null null :!label _label_2)
                  (`GameplayStatics.SpawnSoundAtLocation` "/Game/Audio/Shoot_cue.Shoot_cue" (`SceneComponent.K2_GetComponentLocation` (`self.Muzzle1`)) (struct) 1.0 1.0 0.0 null null)
                  (`GameplayStatics.SpawnEmitterAttached` "/Game/ParticleSystems/MuzzleFlash/ParticleSystems/PS_MuzzleFlash.PS_MuzzleFlash" (`self.BulletSpawn`))
                  (`KismetSystemLibrary.Delay` (`self.FireRate`))
                  (if (and (`self.Sighted`) (not (`/Game/Blueprints/BP_Player.isDead` _asbp_player)) (not (`self.Dead`)) (`self.CanSeePlayer`))
                    (goto _label_2)
                    (else
                      (goto _label :!via `Open`))))))))
        (else
          ;;[1 1 1] Rotate Switching
          (if (`self.Right`)
            (`SceneComponent.K2_AddRelativeRotation` _sphere (struct :`Yaw` 0.5) false false)
            (else
              (`SceneComponent.K2_AddRelativeRotation` _sphere (struct :`Yaw` -0.5) false false)))
          (set `self.TurnCounter` (+ (`self.TurnCounter`) 1.0))
          (if (> (`self.TurnCounter`) (`self.TurnTime`))
            (set `self.TurnCounter` 0.0)
            (`/Engine/EditorBlueprintResources/StandardMacros.FlipFlop`
              (:`A`
                (set `self.Right` false))
              (:`B`
                (set `self.Right` true)))))))))

(fn `CanSeePlayer`
  (returns (ReturnValue :type Boolean))
  (bind _outhit (`KismetSystemLibrary.LineTraceSingleForObjects` :`Start` (`SceneComponent.K2_GetComponentLocation` (`self.BulletSpawn`)) :`End` (`self.K2_GetActorLocation` (`GameplayStatics.GetPlayerPawn` 0)) :`ObjectTypes` (`self.ObjectTypes`) :`DrawTime` 1.0))
  (return (== (`.HitActor` (`GameplayStatics.BreakHitResult` _outhit)) (`GameplayStatics.GetPlayerPawn` 0))))

(fn `Detach Parts`
  (`self.DetachPart` (`self.Cube2`))
  (`self.DetachPart` (`self.Cube1`))
  (`self.DetachPart` (`self.Weapon1`))
  (`self.DetachPart` (`self.Muzzle1`))
  (`self.DetachPart` (`self.Barrel1`))
  (`self.DetachPart` (`self.Arm`))
  (`self.DetachPart` (`self.Base`)))

(fn `DetachPart`
  (params (Mesh :type "StaticMeshComponent Object Reference"))
  (`SceneComponent.K2_DetachFromComponent` Mesh "KeepWorld" "KeepWorld" "KeepWorld" true)
  (`PrimitiveComponent.SetSimulatePhysics` Mesh true)
  (return))

(fn `PointTowardsPlayer`
  (returns (ReturnValue :type "Rotator Structure"))
  (bind _sphere (`self.Sphere`))
  (return (`KismetMathLibrary.RInterpTo` (`SceneComponent.K2_GetComponentRotation` _sphere) (`KismetMathLibrary.FindLookAtRotation` (`SceneComponent.K2_GetComponentLocation` _sphere) (`self.K2_GetActorLocation` (`GameplayStatics.GetPlayerPawn` 0))) 1.0 0.04)))

(fn `UserConstructionScript`)