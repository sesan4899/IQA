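; Player character with mana-fueled shooting and directional dashing, multi-jump, health, and XP leveling.
; Level-ups show an upgrade widget, and AddStats trades stronger damage, fire rate or dash recharge for higher mana costs, or raises health or mana regen.
; Gates pace firing and dashes, timelines drive recoil and blur, and a camera trace sets depth-of-field focus.
; Much logic, including firing, dash, damage and XP, is unconnected to any event here.
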(event `UpdateDoF`
  ;[1 1 1] Automatic depth of field
)

(event `InputAction|StatCheck`
  (params (Key :type "Key Structure"))
  ;[1 1 1] Comment
)

(event `InputAction|Restart`
  (params (Key :type "Key Structure"))
  ;[1 1 1] Restarting
)

(event `InputAction|LevelUp`
  (params (Key :type "Key Structure")))

(event `Recieve Exp`
  (params (Exp :type "Float (double-precision)"))
  ;[1 1 1] Experience Handling
)

(event `Selected PowerUp`
  (bind (_ui _ui_2) (`self.UI`))
  ;[1 1 1] Unpause after level up
  (`Widget.RemoveFromParent` (`.LevelUpUi` (`self.LevelUpUi`)))
  (bind (_direction _blur) (`Timeline|Blur` :!via `PlayFromStart`)
    (:`Update`
      (`self.SetBlur` _ui_2 _blur)
      (`KismetSystemLibrary.Delay` 0.2)
      (`self.SetBlur` _ui_2 0.0))))

(event `self.ReceiveAnyDamage`
  (params (Damage :type "Float (single-precision)") (DamageType :type "DamageType Object Reference") (InstigatedBy :type "Controller Object Reference") (DamageCauser :type "Actor Object Reference"))
  ;[1 1 1] Take Damage
)

(event `Add Stats`
  (params (`Stat string` :type String))
  ;[1 1 1] Add Stats
  (switch `string` `Stat string`
    (:`ManaReg`
      ;[1 1 1] Set Mana
      (set `self.ManaReg` (+ (`self.ManaReg`) 10.0)))
    (:`Damage`
      ;[1 1 1] Set Damage
      (set `self.Damage` (+ (`self.Damage`) 20.0))
      (set `self.AttackCost` (+ (`self.AttackCost`) 5.0)))
    (:`FireRate`
      ;[1 1 1] Set Fire rate
      (set `self.FireRate` (- (`self.FireRate`) 0.1))
      (set `self.AttackCost` (+ (`self.AttackCost`) 5.0)))
    (:`DashReg`
      ;[1 1 1] Set Dash Reg
      (set `self.DashReg` (- (`self.DashReg`) 0.2))
      (set `self.DashCost` (+ (`self.DashCost`) 15.0)))
    (:`Health`
      ;[1 1 1] Set HP
      (set `self.MaxHp` (+ (`self.MaxHp`) 20.0)))))

(event `Dead`
  ;[1 1 1] Dying
)

(event `self.ReceiveTick`
  (params (DeltaSeconds :type "Float (single-precision)")))

(event `self.ReceiveBeginPlay`
  ;[1 1 1] Handle UI
  (bind _returnvalue (`|CreateWidget` null null self))
  (`UserWidget.AddToViewport` _returnvalue 0)
  (set `self.UI` null _returnvalue)
  (bind _returnvalue_2 (`|CreateWidget` null null self))
  (set `self.LevelUpUi` null _returnvalue_2)
  (bind _returnvalue_3 (`|CreateWidget` null null self))
  (set `self.StatScreen` null _returnvalue_3)
  ;[1 1 1] Reset Stats
  (set `self.Mana` (`self.MaxMana`))
  (set `self.Health` (`self.MaxHp`)))

(event `InputAxis|Turn`
  (params (AxisValue :type "Float (single-precision)"))
  ;[1 1 1] Camera Controll
)

(event `InputAxis|LookUp`
  (params (AxisValue :type "Float (single-precision)"))
  ;[1 1 1] Camera Controll
)

(event `InputAction|Forward`
  (params (Key :type "Key Structure"))
  ;[1 1 1] Movement
)

(event `InputAxis|MoveForward`
  (params (AxisValue :type "Float (single-precision)"))
  ;[1 1 1] Movement
  (if (not (`self.Death`))
    (`self.AddMovementInput` (`SceneComponent.GetForwardVector` (`self.CapsuleComponent`)) AxisValue)
    (if (not (`NavMovementComponent.IsFalling` (`self.CharacterMovement`))) :!label _label
      (set `self.FootStepTimer` (+ (`self.FootStepTimer`) (`self.StepSpeed`)) :!label _label_2)
      (if (and (not (`self.Forward Held`)) (not (`self.Backward Held`)) (not (`self.Right Held`)) (not (`self.Left Held`)))
        _
        (elif (>= (`self.FootStepTimer`) (`self.StepLength`))
          (`GameplayStatics.PlaySound2D` null 1.0 1.0 0.0 null null)
          (`GameplayStatics.PlayWorldCameraShake` null (`SceneComponent.K2_GetComponentLocation` (`self.CapsuleComponent`)) 0.0 500.0)
          (set `self.FootStepTimer` 0.0)
          (goto _label_2))))))

(event `InputAction|Backward`
  (params (Key :type "Key Structure"))
  ;[1 1 1] Movement
)

(event `InputAction|Right`
  (params (Key :type "Key Structure"))
  ;[1 1 1] Movement
)

(event `InputAxis|MoveRight`
  (params (AxisValue :type "Float (single-precision)"))
  ;[1 1 1] Movement
  (if (not (`self.Death`))
    (`self.AddMovementInput` (`SceneComponent.GetRightVector` (`self.CapsuleComponent`)) AxisValue)
    (goto _label)))

(event `InputAction|Left`
  (params (Key :type "Key Structure"))
  ;[1 1 1] Movement
)

(event `InputAction|Jump`
  (params (Key :type "Key Structure"))
  ;[1 1 1] Jump / Double Jump
)

(event `self.OnLanded`
  (params (Hit :type "HitResult Structure (by ref)"))
  (bind _charactermovement (`self.CharacterMovement`))
  ;[1 1 1] Jump / Double Jump
  (bind _counter (`/Engine/EditorBlueprintResources/StandardMacros.Do N` (`self.Jumps`) :!via `Reset`)
    (:`Exit`
      (`GameplayStatics.PlaySound2D` null 1.0 1.0 0.0 null null)
      (switch `int` _counter
        (:`1`
          (if (`NavMovementComponent.IsFalling` (`self.CharacterMovement`))
            (`/Engine/EditorBlueprintResources/StandardMacros.IncrementInt` _counter
              (:`  `
                _))
            (else
              (`self.Jump`))))
        (:`2`
          (set `MovementComponent.Velocity` (`KismetMathLibrary.MakeVector` (.x (`MovementComponent.Velocity` _charactermovement)) (.y (`MovementComponent.Velocity` _charactermovement))) _charactermovement)))
      (`self.LaunchCharacter` (0.0 0.0 700.0)))))

(event `InputAction|Dash`
  (params (Key :type "Key Structure")))

(event `self.WallJump.OnComponentBeginOverlap`
  (params (OverlappedComponent :type "PrimitiveComponent Object Reference") (OtherActor :type "Actor Object Reference") (OtherComp :type "PrimitiveComponent Object Reference") (OtherBodyIndex :type Integer) (bFromSweep :type Boolean) (SweepResult :type "HitResult Structure (by ref)")))

(event `self.WallJump.OnComponentEndOverlap`
  (params (OverlappedComponent :type "PrimitiveComponent Object Reference") (OtherActor :type "Actor Object Reference") (OtherComp :type "PrimitiveComponent Object Reference") (OtherBodyIndex :type Integer)))

(event `InputAction|Fire`
  (params (Key :type "Key Structure")))

(fn `UserConstructionScript`
  (`KismetMaterialLibrary.CreateDynamicMaterialInstance` (`PrimitiveComponent.GetMaterial` (`self.Lights`) 0))
  (set `self.EmissiveMaterial` null))