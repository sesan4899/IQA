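; Interactable computer that moves the player through a world "de-res" effect, driven by timelines writing player location and amount to a material parameter collection.
; When powered by StartComputer, use plays the effect, fades out and opens LevelTravelTest.
; Unpowered with a USB enabled, it instead possesses BP_Player after a delay and runs a second effect with input temporarily disabled.
; USBEnabled shows the stick and outlines the screen via custom depth; use clears the outline.
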(event `/Game/Blueprints/BP_Interfaces.Interact`
  (`self.Use`))

(event `StartComputer`
  (set `self.HasElectricity` true)
  (`KismetSystemLibrary.PrintString` "Computer started"))

(event `Use`
  (if (`self.HasElectricity`)
    (`|ExecutionSequence`
      (:`then_0`
        (set `self.isTraveling` true)
        (`KismetMaterialLibrary.SetVectorParameterValue` "/Game/Materials/M_WorldDeRes/PC_WorldDeRes.PC_WorldDeRes" "Location" (`KismetMathLibrary.Conv_VectorToLinearColor` (`self.K2_GetActorLocation` (`GameplayStatics.GetPlayerCharacter` 0))))
        (bind (_direction _newtrack_0) (`Timeline|Timeline_0`)
          (:`Update`
            (`KismetMaterialLibrary.SetScalarParameterValue` "/Game/Materials/M_WorldDeRes/PC_WorldDeRes.PC_WorldDeRes" "Amount" _newtrack_0))
          (:`Finished`
            (`|ExecutionSequence`
              (:`then_0`
                (bind _returnvalue (`|CreateWidget` "/Game/Blueprints/Player/BP_Fade.BP_Fade_C" (`GameplayStatics.GetPlayerController` 0)))
                (set `self.Fade Reference` _returnvalue)
                (`UserWidget.AddToViewport` _returnvalue 0))
              (:`then_1`
                (`/Game/Blueprints/Player/BP_Fade.Fade Out` (`self.Fade Reference`))
                ;[1 1 1] New level
                (`GameplayStatics.OpenLevel` "LevelTravelTest" false)
                (set `self.HasElectricity` false))))))
      (:`then_1`
        (`PrimitiveComponent.SetRenderCustomDepth` (`self.Screen`) false)
        (`KismetArrayLibrary.Array_Clear` (`ActorComponent.ComponentTags` (`self.Screen`)))))
    (else
      (`KismetSystemLibrary.PrintString` "No Electricity")
      (if (`self.HasUSB`)
        (`PrimitiveComponent.SetRenderCustomDepth` (`self.Screen`) false)
        (`KismetArrayLibrary.Array_Clear` (`ActorComponent.ComponentTags` (`self.Screen`)))
        (`KismetMaterialLibrary.SetVectorParameterValue` "/Game/Materials/M_WorldDeRes/PC_WorldDeRes.PC_WorldDeRes" "Location" (`KismetMathLibrary.Conv_VectorToLinearColor` (`self.K2_GetActorLocation` (`GameplayStatics.GetPlayerCharacter` 0))))
        (bind (_direction_2 _newtrack_0_2) (`Timeline|Timeline_2`)
          (:`Update`
            (`KismetMaterialLibrary.SetScalarParameterValue` "/Game/Materials/M_WorldDeRes/PC_WorldDeRes.PC_WorldDeRes" "Amount" _newtrack_0_2)
            (`KismetSystemLibrary.Delay` 6.0)
            (bind _returnvalue_2 (`GameplayStatics.GetActorOfClass` "/Game/Blueprints/Player/BP_Player.BP_Player_C"))
            (`Controller.Possess` (`GameplayStatics.GetPlayerController` 0) _returnvalue_2)
            (`self.DisableInput` (`GameplayStatics.GetPlayerCharacter` 0) (`GameplayStatics.GetPlayerController` 0))
            (`KismetMaterialLibrary.SetVectorParameterValue` "/Game/Materials/M_WorldDeRes/PC_WorldDeRes.PC_WorldDeRes" "Location" (`KismetMathLibrary.Conv_VectorToLinearColor` (`self.K2_GetActorLocation` (`GameplayStatics.GetPlayerCharacter` 0))))
            (bind (_direction_3 _newtrack_0_3) (`Timeline|Timeline_3`)
              (:`Update`
                (`KismetMaterialLibrary.SetScalarParameterValue` "/Game/Materials/M_WorldDeRes/PC_WorldDeRes.PC_WorldDeRes" "Amount" _newtrack_0_3)
                (`KismetSystemLibrary.Delay` 5.0)
                (`self.EnableInput` (`GameplayStatics.GetPlayerCharacter` 0) (`GameplayStatics.GetPlayerController` 0))))))
        (else
          (`KismetSystemLibrary.PrintString` "No USB"))))))

(event `USBEnabled`
  (set `self.HasUSB` true)
  (`SceneComponent.SetVisibility` (`self.USB`) true false)
  (`PrimitiveComponent.SetRenderCustomDepth` (`self.Screen`) true)
  (`KismetArrayLibrary.Array_Add` (`ActorComponent.ComponentTags` (`self.Screen`)) "Newoutline"))

(fn `UserConstructionScript`)