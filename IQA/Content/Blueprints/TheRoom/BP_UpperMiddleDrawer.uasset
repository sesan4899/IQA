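; BP_UpperMiddleDrawer is an interactable drawer in TheRoom that opens or closes on Interact, depending on CanClose.
; A timeline plays or reverses to lerp the mesh's relative location between start and end positions.
; Each timeline update also disables custom depth rendering and clears the mesh's component tags, with nothing here restoring them.
; The update chain flips CanClose after a short delay, in both directions.
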(event `/Game/Blueprints/BP_Interfaces.Interact`
  (if (`self.CanClose`)
    (`self.Close`)
    (else
      (`self.Open`))))

(event `Open`
  (bind (_direction _open) (`Timeline|Timeline_0` :!label _label)
    (:`Update`
      (`SceneComponent.K2_SetRelativeLocation` (`self.StaticMeshComponent`) (`KismetMathLibrary.VLerp` (`self.StartLocation`) (`self.EndLocation`) _open) false false)
      (`PrimitiveComponent.SetRenderCustomDepth` (`self.StaticMeshComponent`) false)
      (`KismetArrayLibrary.Array_Clear` (`ActorComponent.ComponentTags` (`self.StaticMeshComponent`)))
      (`KismetSystemLibrary.Delay` 1.1)
      (if (`self.CanClose`)
        (set `self.CanClose` false)
        (else
          (set `self.CanClose` true))))))

(event `Close`
  (goto _label :!via `Reverse`))

(fn `UserConstructionScript`)