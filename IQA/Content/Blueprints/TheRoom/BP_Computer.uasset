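; Interactable room computer that acts as a portal, to Neon when it has electricity or to Pyramid once its USB is enabled.
; Timelines drive the PC_WorldDeRes parameter collection around the player's location, bracketing a fade, possession of BP_Player and a temporary input lock.
; External events set power and USB state, toggling the screen's outline tag or custom depth.
; FMOD plays transition and startup sounds, the latter followed by the screen light.
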(event `StartComputer`
  (set `self.HasElectricity` true)
  (`KismetArrayLibrary.Array_Add` (`ActorComponent.ComponentTags` (`self.Screen`)) "Newoutline"))

(event `/Game/Blueprints/BP_Interfaces.Interact`
  (`self.Use`))

(event `Use`
  (if (`self.HasElectricity`)
    (`|ExecutionSequence`
      (:`then_0`
        ;[1 1 1] Portal to Neon
        (set `self.isTraveling` true)
        (`KismetMaterialLibrary.SetVectorParameterValue` "/Game/Materials/M_WorldDeRes/PC_WorldDeRes.PC_WorldDeRes" "Location" (`KismetMathLibrary.Conv_VectorToLinearColor` (`self.K2_GetActorLocation` (`GameplayStatics.GetPlayerCharacter` 0))))
        (bind (_direction _newtrack_0) (`Timeline|Timeline_0`)
          (:`Update`
            (`KismetMaterialLibrary.SetScalarParameterValue` "/Game/Materials/M_WorldDeRes/PC_WorldDeRes.PC_WorldDeRes" "Amount" _newtrack_0))
          (:`Finished`
            (`|ExecutionSequence`
              (:`then_0`
                (bind _returnvalue (`|CreateWidget` "/Game/Blueprints/Player/BP_Fade.BP_Fade_C" (`GameplayStatics.GetPlayerController` 0)))
                (set `self.Fade Reference` _returnvalue)
                (`UserWidget.AddToViewport` _returnvalue 0))
              (:`then_1`
                (`/Game/Blueprints/Player/BP_Fade.Fade Out` (`self.Fade Reference`))
                (`KismetSystemLibrary.Delay` 1.1)
                (bind _returnvalue_2 (`GameplayStatics.GetActorOfClass` "/Game/Blueprints/Player/BP_Player.BP_Player_C"))
                (`Controller.Possess` (`GameplayStatics.GetPlayerController` 0) _returnvalue_2)
                (`self.DisableInput` (`GameplayStatics.GetPlayerCharacter` 0) (`GameplayStatics.GetPlayerController` 0))
                (`/Game/Blueprints/Player/BP_Fade.Fade in` (`self.Fade Reference`))
                (`KismetMaterialLibrary.SetVectorParameterValue` "/Game/Materials/M_WorldDeRes/PC_WorldDeRes.PC_WorldDeRes" "Location" (`KismetMathLibrary.Conv_VectorToLinearColor` (`self.K2_GetActorLocation` (`GameplayStatics.GetPlayerCharacter` 0))))
                (`|ExecutionSequence`
                  (:`then_0`
                    (bind (_direction_2 _newtrack_0_2) (`Timeline|Timeline_1`)
                      (:`Update`
                        (`KismetMaterialLibrary.SetScalarParameterValue` "/Game/Materials/M_WorldDeRes/PC_WorldDeRes.PC_WorldDeRes" "Amount" _newtrack_0_2))))
                  (:`then_1`
                    (`KismetSystemLibrary.Delay` 4.0)
                    (`self.EnableInput` (`GameplayStatics.GetPlayerCharacter` 0) (`GameplayStatics.GetPlayerController` 0))
                    (set `self.HasElectricity` false)
                    (set `self.isTraveling` false))))))))
      (:`then_1`
        (`PrimitiveComponent.SetRenderCustomDepth` (`self.Screen`) false)
        (`KismetArrayLibrary.Array_Clear` (`ActorComponent.ComponentTags` (`self.Screen`))))
      (:`then_2`
        (`self.TransitionSound`)))
    (else
      ;[1 1 1] Portal to Pyramid
      (if (`self.HasUSB`)
        (set `self.isTraveling` true)
        (`PrimitiveComponent.SetRenderCustomDepth` (`self.Screen`) false)
        (`KismetArrayLibrary.Array_Clear` (`ActorComponent.ComponentTags` (`self.Screen`)))
        (`KismetMaterialLibrary.SetVectorParameterValue` "/Game/Materials/M_WorldDeRes/PC_WorldDeRes.PC_WorldDeRes" "Location" (`KismetMathLibrary.Conv_VectorToLinearColor` (`self.K2_GetActorLocation` (`GameplayStatics.GetPlayerCharacter` 0))))
        (`self.TransitionSound`)
        (bind (_direction_3 _newtrack_0_3) (`Timeline|Timeline_2`)
          (:`Update`
            (`KismetMaterialLibrary.SetScalarParameterValue` "/Game/Materials/M_WorldDeRes/PC_WorldDeRes.PC_WorldDeRes" "Amount" _newtrack_0_3))
          (:`Finished`
            (`|ExecutionSequence`
              (:`then_0`
                (bind _returnvalue_3 (`|CreateWidget` "/Game/Blueprints/Player/BP_Fade.BP_Fade_C" (`GameplayStatics.GetPlayerController` 0)))
                (set `self.Fade Reference` _returnvalue_3)
                (`UserWidget.AddToViewport` _returnvalue_3 0))
              (:`then_1`
                (`/Game/Blueprints/Player/BP_Fade.Fade Out` (`self.Fade Reference`))
                (`KismetSystemLibrary.Delay` 1.1)
                (bind _returnvalue_4 (`GameplayStatics.GetActorOfClass` "/Game/Blueprints/Player/BP_Player.BP_Player_C"))
                (`Controller.Possess` (`GameplayStatics.GetPlayerController` 0) _returnvalue_4)
                (`self.DisableInput` (`GameplayStatics.GetPlayerCharacter` 0) (`GameplayStatics.GetPlayerController` 0))
                (`/Game/Blueprints/Player/BP_Fade.Fade in` (`self.Fade Reference`))
                (`KismetMaterialLibrary.SetVectorParameterValue` "/Game/Materials/M_WorldDeRes/PC_WorldDeRes.PC_WorldDeRes" "Location" (`KismetMathLibrary.Conv_VectorToLinearColor` (`self.K2_GetActorLocation` (`GameplayStatics.GetPlayerCharacter` 0))))
                (bind (_direction_4 _newtrack_0_4) (`Timeline|Timeline_3`)
                  (:`Update`
                    (`KismetMaterialLibrary.SetScalarParameterValue` "/Game/Materials/M_WorldDeRes/PC_WorldDeRes.PC_WorldDeRes" "Amount" _newtrack_0_4)
                    (`KismetSystemLibrary.Delay` 6.0)
                    (`self.EnableInput` (`GameplayStatics.GetPlayerCharacter` 0) (`GameplayStatics.GetPlayerController` 0))
                    (set `self.HasUSB` false)
                    (set `self.isTraveling` false)))))))))))

(event `TransitionSound`
  (bind _output_get (set `self.FMODAudio` (`self.FMODAudio`)))
  (`FMODBlueprintStatics.PlayEventAttached` "/Game/FMOD/Events/Music/roomEvent.roomEvent" _output_get "None" (0.0 0.0 0.0) "KeepWorldPosition" false true false))

(event `ComputerAudio`
  ;[1 1 1] Light up computer + Sound
  (`KismetSystemLibrary.Delay` 4.0)
  (bind _output_get (set `self.FMODAudio` (`self.FMODAudio`)))
  (`FMODBlueprintStatics.PlayEventAttached` "/Game/FMOD/Events/Computer_Start.Computer_Start" _output_get "None" (0.0 0.0 0.0) "KeepRelativeOffset" false true false)
  (`KismetSystemLibrary.Delay` 0.3)
  (`SceneComponent.SetVisibility` (`Actor.RootComponent` (`self.LightScreen`)) true false))

(event `USBEnabled`
  ;[1 1 1] USB Enable
  (set `self.HasUSB` true)
  (`SceneComponent.SetVisibility` (`self.USB`) true false)
  (`PrimitiveComponent.SetRenderCustomDepth` (`self.Screen`) true)
  (`KismetArrayLibrary.Array_Add` (`ActorComponent.ComponentTags` (`self.Screen`)) "Newoutline"))

(fn `UserConstructionScript`)