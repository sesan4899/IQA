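; BP_ElecBox is an interactable electricity box that powers up the room when used.
; Interacting plays a one-shot FMOD lever sound, switches its indicators from red to green, starts BP_Computer and clears the highlight and tags.
; It makes lamp materials emissive and raises three lights' intensity through a timeline.
; The timeline's Update also calls the ventilation and computer audio on every tick.
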(event `Lever_Electricity`
  (`/Engine/EditorBlueprintResources/StandardMacros.DoOnce` false
    (:`Completed`
      (bind _output_get (set `self.FMODAudio` (`self.FMODAudio`)))
      (`FMODBlueprintStatics.PlayEventAttached` "/Game/FMOD/Events/Lever_Electricity.Lever_Electricity" _output_get "None" (0.0 0.0 0.0) "KeepWorldPosition"))))

(event `Use`
  (`self.Lever_Electricity`)
  (`SceneComponent.SetVisibility` (`self.Green Button`) true false)
  (`SceneComponent.SetVisibility` (`self.Green Light`) true false)
  (`SceneComponent.SetVisibility` (`self.Red Light`) false false)
  (`SceneComponent.SetVisibility` (`self.Red Button`) false false)
  (bind _returnvalue (`GameplayStatics.GetActorOfClass` "/Game/Blueprints/TheRoom/BP_Computer.BP_Computer_C"))
  (`/Game/Blueprints/TheRoom/BP_Computer.StartComputer` _returnvalue)
  (for _array_element (`self.Lamps`)
    (`PrimitiveComponent.SetMaterial` (`self.GetComponentByClass` _array_element "/Script/Engine.PrimitiveComponent") 1 "/Game/ContentPacks/Bunker/Materials/M_emisisve.M_emisisve")
    (bind (_direction _intensity) (`Timeline|LightIntensity`)
      (:`Update`
        (`LightComponent.SetIntensity` (`self.GetComponentByClass` (`|GetArrayItem` (`self.Lights`)) "/Script/Engine.LightComponent") (`KismetMathLibrary.Lerp` (`self.StartIntensity`) (`self.EndIntensity`) _intensity))
        (`LightComponent.SetIntensity` (`self.GetComponentByClass` (`|GetArrayItem` (`self.Lights`) 1) "/Script/Engine.LightComponent") (`KismetMathLibrary.Lerp` (`self.StartIntensity`) (`self.EndIntensity`) _intensity))
        (`LightComponent.SetIntensity` (`self.GetComponentByClass` (`|GetArrayItem` (`self.Lights`) 2) "/Script/Engine.LightComponent") (`KismetMathLibrary.Lerp` (`self.StartIntensity`) (`self.EndIntensity`) _intensity))
        (bind _asbp_ventilation (cast `/Game/Blueprints/TheRoom/BP_Ventilation` (`self.Ventilation`)))
        (`/Game/Blueprints/TheRoom/BP_Ventilation.VentAudio` _asbp_ventilation)
        (bind _asbp_computer (cast `/Game/Blueprints/TheRoom/BP_Computer` (`self.Computer`)))
        (`/Game/Blueprints/TheRoom/BP_Computer.ComputerAudio` _asbp_computer)))))

(event `/Game/Blueprints/BP_Interfaces.Interact`
  (`self.Use`)
  (`self.HasInteracted`))

(event `HasInteracted`
  (`PrimitiveComponent.SetRenderCustomDepth` (`self.StaticMesh`) false)
  (`KismetArrayLibrary.Array_Clear` (`ActorComponent.ComponentTags` (`self.StaticMesh`))))

(fn `UserConstructionScript`)