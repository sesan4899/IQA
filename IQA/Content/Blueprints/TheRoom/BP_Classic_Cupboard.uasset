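; BP_Classic_Cupboard is an interactable cupboard that swings its left and right doors open and closed.
; Interact calls Open or Close based on CanClose, which plays or reverses one timeline.
; Timeline updates lerp each door's relative rotation from a shared start rotation to its own end rotation.
; CanClose flips after a Delay on the update path rather than on the timeline's Finished pin.
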(event `/Game/Blueprints/BP_Interfaces.Interact`
  (if (`self.CanClose`)
    (`self.Close`)
    (else
      (`self.Open`))))

(event `Open`
  (bind (_direction _doorrotation) (`Timeline|Timeline_0` :!label _label)
    (:`Update`
      (`|ExecutionSequence`
        (:`then_0`
          (`SceneComponent.K2_SetRelativeRotation` (`self.SM_Classic_Cupboard_Door_Right`) (`KismetMathLibrary.RLerp` (`self.StartRotation`) (`self.EndRotationRight`) _doorrotation) false false))
        (:`then_1`
          (`SceneComponent.K2_SetRelativeRotation` (`self.SM_Classic_Cupboard_Door_Left`) (`KismetMathLibrary.RLerp` (`self.StartRotation`) (`self.EndRotation`) _doorrotation) false false)
          (`KismetSystemLibrary.Delay` 1.1)
          (if (`self.CanClose`)
            (set `self.CanClose` false)
            (else
              (set `self.CanClose` true))))))))

(event `Close`
  (goto _label :!via `Reverse`))

(fn `UserConstructionScript`)