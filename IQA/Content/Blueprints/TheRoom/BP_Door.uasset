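; BP_Door is a door Blueprint that swings open when interacted with, but only after its knob has been attached.
; AddKnob reveals the DoorKnob component and sets CanOpen, which gates the Interact event.
; OpenDoor plays a timeline that lerps the StaticMesh relative rotation from StartRotation to EndRotation.
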(event `AddKnob`
  (`SceneComponent.SetVisibility` (`self.DoorKnob`) true false)
  (set `self.CanOpen` true))

(event `/Game/Blueprints/BP_Interfaces.Interact`
  (if (`self.CanOpen`)
    (`self.OpenDoor`)))

(event `OpenDoor`
  (bind (_direction _doorrotation) (`Timeline|Timeline_0`)
    (:`Update`
      (`SceneComponent.K2_SetRelativeRotation` (`self.StaticMesh`) (`KismetMathLibrary.RLerp` (`self.Start Rotation`) (`self.End Rotation`) _doorrotation) false false))))

(fn `UserConstructionScript`)